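; SocketManager is a Blueprint that rotates a Chair actor in response to rotation messages from a Socket.IO server.
; On BeginPlay it binds the "new rotation" event on the root namespace and prints connection and disconnection status in Portuguese.
; Each event's numeric payload becomes the target yaw, and a timeline lerps the chair there by the shortest path, keeping pitch and roll.
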(event OnConnected(SocketIOClient)
  (params (SessionId :type String))
  (Development|PrintString "Conexão estabelecida!"))

(event OnDisconnected(SocketIOClient)
  (params (Reason :type ESIOConnectionCloseReason%20Enum :default "CLOSE_REASON_NORMAL"))
  (Development|PrintString (Utilities|String|Append "Desconectado: " (Utilities|String|ToString(Byte) Reason))))

(event OnEvent(SocketIOClient)
  (params (Event :type String) (MessageJson :type SIO%20Json%20Value%20Object%20Reference))
  (if (Utilities|Enum|Equal(Enum) Event "new rotation")
    (bind _output_get (Variables|Default|SetChairCurrentRotation (Transformation|GetActorRotation (Variables|Default|GetChair))))
    (bind _alpha (Timeline|RotationTimeline PlayFromStart)
      (:Update
        (Transformation|SetActorRotation (Variables|Default|GetChair) (Math|Rotator|Lerp(Rotator) (Variables|Default|GetChairCurrentRotation) (Math|Rotator|MakeRotator (.Roll (Math|Rotator|BreakRotator _output_get)) (.Pitch (Math|Rotator|BreakRotator _output_get)) (Class|SIOJsonValue|AsNumber MessageJson)) _alpha true))))))

(event EventBeginPlay
  (Class|SocketIOClientComponent|BindEvent (Variables|Default|GetSocketIOClient) "new rotation" "/"))

(fn ConstructionScript)