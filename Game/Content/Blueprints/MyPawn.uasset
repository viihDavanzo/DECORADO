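; Player pawn for a mouse-driven object placement editor with Construction and Edit modes, each with its own widget.
; A per-tick camera-to-cursor trace positions the preview mesh or dragged object, whose collision is disabled, and detects Objects_Base actors for custom-depth highlighting.
; Construction spawns the previewed class, chosen by key from an array.
; Edit selects, drags and deletes objects; both modes rotate in yaw and step through each object's material list.
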(event EventTick
  (params (DeltaSeconds :type Float%20%28single-precision%29))
  (bind _selectedobject (Variables|Default|GetSelectedObject))
  ;[0 0 0] Line trace que cuida da posição dos objetos relativos à posição do mouse e se há algum objeto disponível para interação
  ;;[1 0 0] Event Tick
  (bind (_outhit _returnvalue) (Collision|LineTraceByChannel (Camera|GetCameraLocation (Game|GetPlayerCameraManager 0)) (Utilities|MousePositiontoWorldSpace (Variables|Default|GetMaxRange)) "TraceTypeQuery1" true 0 "ForOneFrame"))
  (if _returnvalue
    (Variables|Default|SetMouseLocation (.Location (Collision|BreakHitResult _outhit)))
    (if (Variables|Default|GetCanDrag)
      (Collision|SetActorEnableCollision _selectedobject false)
      (Transformation|SetWorldLocation (Variables|/Script/Engine.Actor|GetRootComponent _selectedobject) (Variables|Default|GetMouseLocation) false false)
      (else
        (Transformation|SetWorldLocation (Variables|Default|GetCurrentMesh) (Variables|Default|GetMouseLocation) false false)
        (if (and (not (Variables|Default|GetConstructionMode)) (Utilities|ClassIsChildOf (Utilities|GetClass (.HitActor (Collision|BreakHitResult _outhit))) "/Game/Blueprints/Objects_Base.Objects_Base_C"))
          (Variables|Default|SetObjectAvailable true)
          (bind _output_get (Variables|Default|SetAvailableObject (.HitActor (Collision|BreakHitResult _outhit))))
          (CallFunction|SetCustomDepthRender _output_get true)
          (Variables|Default|SetLastSeenObject _output_get)
          (else
            (Variables|Default|SetObjectAvailable false)
            (if (Variables|Default|GetObjectSelected)
              (if (!= (Variables|Default|GetLastSeenObject) (Variables|Default|GetSelectedObject))
                (CallFunction|SetCustomDepthRender (Variables|Default|GetLastSeenObject) false))
              (else
                (CallFunction|SetCustomDepthRender (Variables|Default|GetAvailableObject) false)
                (Variables|Default|SetAvailableObject 0)))))))))

(event EventBeginPlay
  ;[1 0 0] Event BeginPlay
  (bind _returnvalue (UserInterface|CreateWidget "/Game/UI/ObjectsMenu.ObjectsMenu_C")) ; Cria a Widget "Objects Menu".
  (bind _output_get (Variables|UI|SetObjectsMenu_Ref _returnvalue)) ; Guarda ela em uma variável.
  (UserInterface|Viewport|AddtoViewport _output_get 0) ; A adiciona à Viewport
  (CallFunction|ChangeMeshandStoreMaterials)
  (bind _returnvalue_2 (UserInterface|CreateWidget "/Game/UI/ConstructionMode.ConstructionMode_C")) ; Cria a Widget "Construction Mode".
  (bind _output_get_2 (Variables|UI|SetConstructionMode_Ref _returnvalue_2))
  (UserInterface|Viewport|AddtoViewport _output_get_2 0)
  (bind _returnvalue_3 (UserInterface|CreateWidget "/Game/UI/EditMode.EditMode_C")) ; Cria a Widget "Edit Mode".
  (Variables|UI|SetEditMode_Ref _returnvalue_3))

(event Input|ActionEvents|InputActionConstructionMode
  (params (Key :type Key%20Structure))
  ;[0 0 0] Mudança entre os modos de edição
  (:Pressed
    (if (not (Variables|Default|GetConstructionMode))
      (if (Variables|Default|GetObjectSelected)
        (Variables|Default|SetObjectSelected false)
        (Variables|Default|SetObjectAvailable false)
        (CallFunction|SetCustomDepthRender (Variables|Default|GetSelectedObject) false)
        (Variables|Default|SetAvailableObject 0)
        (CallFunction|EnableConstructionMode)
        (else
          (CallFunction|EnableConstructionMode))))))

(event Input|ActionEvents|InputActionEditMode
  (params (Key :type Key%20Structure))
  ;[0 0 0] Mudança entre os modos de edição
  (:Pressed
    (if (Variables|Default|GetConstructionMode)
      (Variables|Default|SetConstructionMode false)
      (Components|StaticMesh|SetStaticMesh (Variables|Default|GetCurrentMesh) 0)
      (Default|CallSetRenderText "MODO DE EDIÇÃO")
      (Widget|RemovefromParent (Variables|UI|GetConstructionMode_Ref))
      (UserInterface|Viewport|AddtoViewport (Variables|UI|GetEditMode_Ref) 0))))

(event Input|ActionEvents|InputActionDelete
  (params (Key :type Key%20Structure))
  ;[0 0 0] Deleta o objeto selecionado no modo de edição
  (:Pressed
    (if (not (Variables|Default|GetConstructionMode))
      (CallFunction|DestroySelectedObject))))

(event Input|ActionEvents|InputActionInteract
  (params (Key :type Key%20Structure))
  ;[0 0 0] Interação com objetos em ambos os modos de edição
  ;;[1 0 0] Input Action Interact
  (:Pressed
    (if (Variables|Default|GetConstructionMode) ; Está no modo de Construção?
      (bind _returnvalue (Game|SpawnActorfromClass (Utilities|GetClass (Utilities|Array|Get(acopy) (Variables|Arrays|GetObjectsBaseArray) (Variables|Default|GetObjectID))) (Transformation|GetWorldTransform (Variables|Default|GetCurrentMesh)) "Undefined" 0 0)) ; Cria um objeto da mesma classe mostrada
      (Rendering|Material|SetMaterial (Variables|/Game/Blueprints/Objects_Base.Objects_Base_C|GetStaticMesh _returnvalue) 0 (Utilities|Array|Get(acopy) (Variables|Arrays|GetMaterialInstancesArray) (Variables|Default|GetMaterialID))) ; Muda o material do objeto para o mesmo mostrado
      (Development|SetHiddeninGame (Variables|/Game/Blueprints/Objects_Base.Objects_Base_C|GetStaticMesh _returnvalue) false false) ; Mostra a mesh (escondida por padrão)
      (elif (Variables|Default|GetObjectAvailable) ; O objeto está disponível?
        (if (Variables|Default|GetObjectSelected) ; Já existe um objeto selecionado?
          (if (== (Variables|Default|GetSelectedObject) (Variables|Default|GetAvailableObject)) ; O objeto selecionado é igual ao objeto disponível?
            (Variables|Default|SetCanDrag true) ; Pode ser arrastado
            (else
              (CallFunction|SetCustomDepthRender (Variables|Default|GetSelectedObject) false) ; Desliga a borda de seleção
              (Variables|Default|SetSelectedObject (Variables|Default|GetAvailableObject)) ; O objeto disponível se torna o objeto selecionado
              (bind _materialinstances (CallFunction|GetObjectStructureandStaticMesh (Variables|Default|GetSelectedObject))) ; Pega a Structure e a Static Mesh do objeto selecionado
              (bind _output_get (Variables|Arrays|SetMaterialInstancesArray _materialinstances)) ; Guarda sua Array de materiais
              (for (_array_element _array_index) _output_get ; Compara os materiais da Array com o da mesh do objeto
                (if (== _array_element (Rendering|Material|GetMaterial (Variables|/Game/Blueprints/Objects_Base.Objects_Base_C|GetStaticMesh (.AsObjects%20Base (Utilities|Casting|CastToObjects_Base (Variables|Default|GetSelectedObject)))) 0)) ; Caso os materiais sejam iguais
                  (Variables|Default|SetMaterialID _array_index) ; Atualiza a ID do material (para que haja um ciclo perfeito)
                ))))
          (else
            (Variables|Default|SetObjectSelected true) ; Agora há um objeto selecionado
            (Variables|Default|SetSelectedObject (Variables|Default|GetAvailableObject)) ; O objeto disponível se torna o objeto selecionado
          ))
        (else
          (CallFunction|SetCustomDepthRender (Variables|Default|GetSelectedObject) false) ; Desliga a borda de seleção
          (Variables|Default|SetSelectedObject 0) ; Reset o objeto selecionado
          (Variables|Default|SetObjectSelected false) ; Não há mais objeto selecionado
        ))))
  (:Released
    (if (Variables|Default|GetCanDrag) ; O objeto pode ser arrastado?
      (Variables|Default|SetCanDrag false) ; O objeto agora não pode mais ser arrastado
      (Collision|SetActorEnableCollision (Variables|Default|GetSelectedObject) true) ; Liga a colisão do objeto selecionado
    )))

(event Input|AxisEvents|InputAxisRotation
  (params (AxisValue :type Float%20%28single-precision%29))
  (bind _selectedobject (Variables|Default|GetSelectedObject))
  (bind _rootcomponent (Variables|/Script/Engine.Actor|GetRootComponent _selectedobject))
  ;[0 0 0] Rotação de objetos em ambos os modos de edição
  (if (Variables|Default|GetConstructionMode)
    (Transformation|SetWorldRotation (Variables|Default|GetCurrentMesh) (Utilities|RotateObjectinZ (Variables|Default|GetCurrentMesh) AxisValue) false false)
    (elif (Variables|Default|GetObjectSelected)
      (Utilities|IsValid _selectedobject
        (:Is%20Valid
          (Transformation|SetWorldRotation _rootcomponent (Utilities|RotateObjectinZ _rootcomponent AxisValue) false false))))))

(event Input|KeyboardEvents|Up
  (params (Key :type Key%20Structure))
  ;[0 1 0] Muda os materiais em ambos os modos de edição
  (:Pressed
    (if (Variables|Default|GetConstructionMode)
      (bind _materialid (Utilities|NextMaterialID))
      (Rendering|Material|SetMaterial (Variables|Default|GetCurrentMesh) 0 (Utilities|Array|Get(acopy) (Variables|Arrays|GetMaterialInstancesArray) _materialid))
      (elif (Variables|Default|GetObjectSelected)
        (bind (_mesh _materialinstances _staticmesh) (CallFunction|GetObjectStructureandStaticMesh (Variables|Default|GetSelectedObject)))
        (bind _materialid_2 (Utilities|NextMaterialID))
        (Rendering|Material|SetMaterial _staticmesh 0 (Utilities|Array|Get(acopy) _materialinstances _materialid_2))))))

(event Input|KeyboardEvents|Down
  (params (Key :type Key%20Structure))
  ;[0 1 0] Muda os materiais em ambos os modos de edição
  (:Pressed
    (if (Variables|Default|GetConstructionMode)
      (bind _materialid (Utilities|LastMaterialID))
      (Rendering|Material|SetMaterial (Variables|Default|GetCurrentMesh) 0 (Utilities|Array|Get(acopy) (Variables|Arrays|GetMaterialInstancesArray) _materialid))
      (elif (Variables|Default|GetObjectSelected)
        (bind (_mesh _materialinstances _staticmesh) (CallFunction|GetObjectStructureandStaticMesh (Variables|Default|GetSelectedObject)))
        (bind _materialid_2 (Utilities|LastMaterialID))
        (Rendering|Material|SetMaterial _staticmesh 0 (Utilities|Array|Get(acopy) _materialinstances _materialid_2))))))

(event Input|KeyboardEvents|AnyKey
  (params (Key :type Key%20Structure))
  ;[0 0 0] Mudança de objetos no nodo de construção
  (:Pressed
    (if (Variables|Default|GetConstructionMode)
      (if (Utilities|Array|ContainsItem (Variables|Arrays|GetKeysArray) Key)
        (Variables|Default|SetObjectID (- (Math|Conversions|ToInteger(Byte) (Utilities|String|ToString(Text) (Class|KismetInputLibrary|KeyGetDisplayName Key))) 1))
        (Default|Fadein (Variables|UI|GetObjectsMenu_Ref))
        (CallFunction|ChangeMeshandStoreMaterials)
        (Variables|Default|SetMaterialID 0)))))

(fn ConstructionScript)

(fn ChangeMeshandStoreMaterials
  (bind _objectid (Variables|Default|GetObjectID))
  (bind _objectsbasearray (Variables|Arrays|GetObjectsBaseArray))
  (bind _materialinstancesarray (Variables|Arrays|GetMaterialInstancesArray))
  (bind _output (Utilities|Array|Get(acopy) _objectsbasearray _objectid))
  (bind _objectstructure (Variables|/Game/Blueprints/Objects_Base.Objects_Base_C|GetObjectStructure _output))
  (bind (_name _mesh _materialinstances) (Utilities|Struct|BreakObjects_Structure _objectstructure))
  (Utilities|Array|Clear (Variables|Arrays|GetMaterialInstancesArray))
  (for _array_element _materialinstances
    (Utilities|Array|Add _materialinstancesarray _array_element)
    (Components|StaticMesh|SetStaticMesh (Variables|Default|GetCurrentMesh) _mesh)
    (Rendering|Material|SetMaterial (Variables|Default|GetCurrentMesh) 0 (Utilities|Array|Get(acopy) _materialinstancesarray))))

(fn SetCustomDepthRender
  (params (Object :type Object%20Object%20Reference) (bValue :type Boolean))
  (Utilities|IsValid Object
    (:Is%20Valid
      (bind _asobjects_base (Utilities|Casting|CastToObjects_Base Object))
      (Rendering|SetRenderCustomDepth (Variables|/Game/Blueprints/Objects_Base.Objects_Base_C|GetStaticMesh _asobjects_base) bValue))))

(fn EnableConstructionMode
  (Variables|Default|SetConstructionMode true)
  (Components|StaticMesh|SetStaticMesh (Variables|Default|GetCurrentMesh) (.Mesh (Utilities|Struct|BreakObjects_Structure (Variables|/Game/Blueprints/Objects_Base.Objects_Base_C|GetObjectStructure (Utilities|Array|Get(acopy) (Variables|Arrays|GetObjectsBaseArray) (Variables|Default|GetObjectID))))))
  (Default|CallSetRenderText "MODO DE CONSTRUÇÃO")
  (Widget|RemovefromParent (Variables|UI|GetEditMode_Ref))
  (UserInterface|Viewport|AddtoViewport (Variables|UI|GetConstructionMode_Ref) 0))

(fn GetObjectStructureandStaticMesh
  (params (Object :type Object%20Object%20Reference))
  (bind _asobjects_base (Utilities|Casting|CastToObjects_Base Object))
  (bind _objectstructure (Variables|/Game/Blueprints/Objects_Base.Objects_Base_C|GetObjectStructure _asobjects_base))
  (bind (_name _mesh _materialinstances) (Utilities|Struct|BreakObjects_Structure _objectstructure))
  (return _mesh _materialinstances (Variables|/Game/Blueprints/Objects_Base.Objects_Base_C|GetStaticMesh _asobjects_base)))

(fn DestroySelectedObject
  (bind _output_get (LocalVariables|SetDestroyedObject (Variables|Default|GetSelectedObject)))
  (Actor|DestroyActor _output_get)
  (Variables|Default|SetSelectedObject 0))